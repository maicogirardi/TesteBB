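; BP_Obras is an actor that displays a cycle of works (obras) on one mesh component, with a name and description for each.
; On BeginPlay it registers itself as the Object on BP_BBPlayerController and starts at the first entry.
; NextObj and PrevObj step a wrapping index through parallel mesh, name and description arrays.
; Each step swaps the static mesh, fills the controller's MainUI text and resets the actor's rotation to zero.
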(event Custom|PrevObj
  (if (> (Variables|Default|GetActualIdx) 0)
    (Math|Integer|DecrementInt (Variables|Default|GetActualIdx)
      (:%20%20
        _))
    (else
      (Variables|Default|SetActualIdx (- (Utilities|Array|Length (Variables|Default|GetObras)) 1))))
  (CallFunction|ChangeMeshandText)
  (CallFunction|ResetRotation))

(event Custom|NextObj
  (if (< (Variables|Default|GetActualIdx) (- (Utilities|Array|Length (Variables|Default|GetObras)) 1))
    (Math|Integer|IncrementInt (Variables|Default|GetActualIdx)
      (:%20%20
        _))
    (else
      (Variables|Default|SetActualIdx 0)))
  (CallFunction|ChangeMeshandText)
  (CallFunction|ResetRotation))

(event Custom|ChangeMeshAndText
  (Components|StaticMesh|SetStaticMesh (Variables|Default|GetObject) (Utilities|Array|Get(acopy) (Variables|Default|GetObras) (Variables|Default|GetActualIdx)))
  (Default|PopulateText (Variables|/Game/GameBPs/BP_BBPlayerController.BP_BBPlayerController_C|GetMainUI (Variables|Default|GetPlayerCharacter)) (Utilities|Array|Get(acopy) (Variables|Default|GetNames) (Variables|Default|GetActualIdx)) (Utilities|Array|Get(acopy) (Variables|Default|GetDescriptions) (Variables|Default|GetActualIdx))))

(event Custom|ResetRotation
  (Transformation|SetActorRotation "0, 0, 0"))

(event EventBeginPlay
  (bind _asbp_bbplayer_controller (Utilities|Casting|CastToBP_BBPlayerController (Game|GetPlayerController 0)))
  (bind _output_get (Variables|Default|SetPlayerCharacter _asbp_bbplayer_controller))
  (Variables|/Game/GameBPs/BP_BBPlayerController.BP_BBPlayerController_C|SetObject _output_get self)
  (Variables|Default|SetActualIdx 0))

(fn ConstructionScript)