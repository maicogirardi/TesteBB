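; BP_BBPlayerController is a player controller for inspecting a 3D object with zoom and drag rotation.
; On BeginPlay it shows the cursor, creates the main UI and moves the character's spring arm to the Object.
; Gates on Tick rotate the Object from mouse deltas while Drag is held; the touch path, marked WIP, uses raw touch location.
; Other events forward next/previous calls to the Object, toggle the config widget and switch mute sound mixes.
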(event Custom|PrevObj
  (Default|PrevObj (Variables|Default|Getobject)))

(event Custom|NextObj
  (Default|NextObj (Variables|Default|Getobject)))

(event Custom|AddConfigUI
  (bind _returnvalue (UserInterface|CreateWidget "/Game/Widgets/UMG_Config.UMG_Config_C"))
  (bind _output_get (Variables|Default|SetConfigUI _returnvalue))
  (UserInterface|Viewport|AddtoViewport _output_get 0))

(event Custom|RemoveConfigUI
  (Widget|RemovefromParent (Variables|Default|GetConfigUI)))

(event Custom|SaveConfigs
  (params (bHasSound :type Boolean))
  (bind _output_get (Variables|Default|SetbHasSound bHasSound))
  (if _output_get
    (Class|GameplayStatics|SetBaseSoundMix "/Game/Sounds/SFx_UnMute.SFx_UnMute")
    (else
      (Class|GameplayStatics|SetBaseSoundMix "/Game/Sounds/SFx_Mute.SFx_Mute"))))

(event Custom|AddMainUI
  (bind _returnvalue (UserInterface|CreateWidget "/Game/Widgets/UMG_Main.UMG_Main_C"))
  (bind _output_get (Variables|Default|SetMainUI _returnvalue))
  (UserInterface|Viewport|AddtoViewport _output_get 0))

(event Custom|ChangeCamPosition
  (Transformation|SetWorldLocation (Variables|Default|GetBB_Spring%20Arm) (Transformation|GetActorLocation (Variables|Default|GetObject)) true true))

(event EventBeginPlay
  (bind _asbp_bbcharacter (Utilities|Casting|CastToBP_BBCharacter (Game|GetPlayerCharacter 0)))
  (Variables|Default|SetBB_Character _asbp_bbcharacter)
  (Variables|Default|SetbShowMouseCursor true)
  (Variables|Default|SetBB_Spring%20Arm (Variables|/Game/GameBPs/BP_BBCharacter.BP_BBCharacter_C|GetSpringArm (Variables|Default|GetBB_Character)))
  (Class|GameplayStatics|SetBaseSoundMix "/Game/Sounds/SFx_UnMute.SFx_UnMute")
  (CallFunction|ChangeCamPosition)
  (CallFunction|AddMainUI))

(event EventTick
  (params (DeltaSeconds :type Float%20%28single-precision%29))
  (bind (_locationx _locationy) (Class|PlayerController|GetInputTouchState "Touch1"))
  (bind (_deltax _deltay) (Class|PlayerController|GetInputMouseDelta))
  (Utilities|FlowControl|Sequence
    (:then_0
      (Utilities|FlowControl|Gate true
        (:Exit
          (Class|Actor|AddActorWorldRotation (Variables|Default|GetObject) (Math|Rotator|MakeRotator 0.0 (* (* _deltay (Variables|Default|GetRotationFactor)) -1.0) (* (* (Variables|Default|GetRotationFactor) _deltax) -1.0)))
          (Default|RestartShadow (Variables|Default|GetObject)))))
    (:then_1
      ;[1 1 1] WIP
      (Utilities|FlowControl|Gate true
        (:Exit
          (Class|Actor|AddActorWorldRotation (Variables|Default|GetObject) (Math|Rotator|MakeRotator 0.0 (* (* _locationy (Variables|Default|GetRotationFactor)) -1.0) (* (* (Variables|Default|GetRotationFactor) _locationx) -1.0))))))))

(event Input|ActionEvents|InputActionDrag
  (params (Key :type Key%20Structure :default "None"))
  (bind (_deltax _deltay) (Class|PlayerController|GetInputMouseDelta))
  (:Pressed
    (Utilities|IsValid (Variables|Default|GetObject)
      (:Is%20Valid
        (Utilities|FlowControl|Gate true) ; enters at Open
      )))
  (:Released
    (Utilities|FlowControl|Gate true) ; enters at Close
  ))

(event Input|AxisEvents|InputAxisZoom
  (params (AxisValue :type Float%20%28single-precision%29))
  (Variables|/Script/Engine.SpringArmComponent|SetTargetArmLength (Variables|Default|GetBB_Spring%20Arm) (Math|Float|Clamp(Float) (+ (* (* AxisValue -1.0) (Variables|Default|GetZoomFactor)) (Variables|/Script/Engine.SpringArmComponent|GetTargetArmLength (Variables|Default|GetBB_Spring%20Arm))) (Variables|Default|GetMinZoom) (Variables|Default|GetMaxZoom))))

(event Input|TouchEvents|InputTouch
  (params (Location :type Vector) (FingerIndex :type ETouchIndex%20Enum))
  (bind (_locationx _locationy) (Class|PlayerController|GetInputTouchState "Touch1"))
  ;[1 1 1] WIP
  (:Pressed
    (Utilities|IsValid (Variables|Default|GetObject)
      (:Is%20Valid
        (Utilities|FlowControl|Gate true) ; enters at Open
      )))
  (:Released
    (Utilities|FlowControl|Gate true) ; enters at Close
  ))

(fn ConstructionScript)